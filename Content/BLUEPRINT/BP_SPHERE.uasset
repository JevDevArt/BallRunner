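; BP_SPHERE is a player-controlled rolling ball that restarts the current level when it takes any damage.
; Both movement axes feed one mass-independent torque on the Sphere, scaled by MULTIPLY.
; Damage fades the camera out with a bonk sound, then reopens the level after a short delay.
; BeginPlay fades in with a sound, and R replays that intro without reloading.
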(event Game|Damage|EventAnyDamage
  (params (Damage :type Float%20%28single-precision%29) (DamageType :type Damage%20Type%20Object%20Reference) (InstigatedBy :type Controller%20Object%20Reference) (DamageCauser :type Actor%20Object%20Reference))
  (CameraFades|StartCameraFade :self (Game|GetPlayerCameraManager 0) :ToAlpha 1.0 :Duration 0.7 :bHoldWhenFinished true)
  (Audio|PlaySound2D "/Game/SOUND/Funny_Bonk.Funny_Bonk" 0.4 1.0 0.0 0 0)
  (Utilities|FlowControl|Delay 1.0)
  (bind _returnvalue (Game|GetCurrentLevelName true))
  (Game|OpenLevel(byName) (Utilities|String|StringToName _returnvalue)))

(event EventBeginPlay
  (CameraFades|StartCameraFade :self (Game|GetPlayerCameraManager 0) :FromAlpha 1.0 :Duration 1.5 :bHoldWhenFinished true)
  (Audio|PlaySound2D "/Game/SOUND/Blushing_.Blushing_" 1.0 1.0 0.0 0 0))

(event Input|AxisEvents|InputAxisMoveForwardBack
  (params (AxisValue :type Float%20%28single-precision%29))
  (Class|PrimitiveComponent|AddTorqueinRadians (Variables|Default|GetSphere) (Math|Vector|MakeVector (* (stale Input|AxisEvents|InputAxisMoveLeftRight AxisValue) (Variables|Default|GetMULTIPLY)) (* AxisValue (Variables|Default|GetMULTIPLY)) 0.0) "None" true))

(event Input|AxisEvents|InputAxisMoveLeftRight
  (params (AxisValue :type Float%20%28single-precision%29))
  (Class|PrimitiveComponent|AddTorqueinRadians (Variables|Default|GetSphere) (Math|Vector|MakeVector (* AxisValue (Variables|Default|GetMULTIPLY)) (* (stale Input|AxisEvents|InputAxisMoveForwardBack AxisValue) (Variables|Default|GetMULTIPLY)) 0.0) "None" true))

(event Input|KeyboardEvents|R
  (params (Key :type Key%20Structure :default "None"))
  (:Pressed
    (CameraFades|StartCameraFade :self (Game|GetPlayerCameraManager 0) :FromAlpha 1.0 :Duration 1.5 :bHoldWhenFinished true)
    (Audio|PlaySound2D "/Game/SOUND/Blushing_.Blushing_" 1.0 1.0 0.0 0 0)))

(fn ConstructionScript)