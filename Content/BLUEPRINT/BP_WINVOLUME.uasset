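; BP_WINVOLUME is a level-exit trigger that completes the level once all crystal collectibles are gone.
; On box overlap, with no actor filter, it searches for remaining BP_COLLECTIBLE and BP_COLLECTIBLE_02 actors and prints a missing-crystals message if any exist.
; Otherwise it fades the camera, plays an explosion sound and, after a delay, opens the next level in LEVELNAMES.
; On the final level it prints a game-over message instead.
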(event OnComponentBeginOverlap(Box)
  (params (OverlappedComponent :type Primitive%20Component%20Object%20Reference) (OtherActor :type Actor%20Object%20Reference) (OtherComp :type Primitive%20Component%20Object%20Reference) (OtherBodyIndex :type Integer) (bFromSweep :type Boolean) (SweepResult :type Hit%20Result%20Structure%20%28by%20ref%29))
  (bind _returnvalue (CallFunction|AllActors))
  (if _returnvalue
    (Development|PrintString "BRAK KRYSZTAŁÓW")
    (else
      (CameraFades|StartCameraFade :self (Game|GetPlayerCameraManager 0) :ToAlpha 1.0 :Duration 0.7 :bHoldWhenFinished true)
      (Audio|PlaySound2D "/Game/StarterContent/Audio/Explosion01.Explosion01" 0.4 1.0 0.0 0 0)
      (Utilities|FlowControl|Delay 1.0)
      (CallFunction|CompleteLevel))))

(fn ConstructionScript)

(fn GetCurrentLevelIndex
  (bind _returnvalue (Game|GetCurrentLevelName true))
  (return (Utilities|Array|FindItem (Variables|Default|GetLEVEL_NAMES) _returnvalue)))

(fn GetNextLevelName
  (return (Utilities|Array|Get(acopy) (Variables|Default|GetLEVEL_NAMES) (+ (CallFunction|GetCurrentLevelIndex) 1))))

(fn LoadNextLevel
  (Game|OpenLevel(byName) (Utilities|String|StringToName (CallFunction|GetNextLevelName))))

(fn IsFinalLevel
  (return (== (CallFunction|GetCurrentLevelIndex) (Utilities|Array|LastIndex (Variables|Default|GetLEVEL_NAMES)))))

(fn CompleteLevel
  (if (CallFunction|IsFinalLevel)
    (Development|PrintString "KONIEC GRY WOOOOW")
    (else
      (CallFunction|LoadNextLevel))))

(fn AllActors
  (bind _outactors (Actor|GetAllActorsOfClass "/Game/BLUEPRINT/BP_COLLECTIBLE_02.BP_COLLECTIBLE_02_C"))
  (bind _outactors_2 (Actor|GetAllActorsOfClass "/Game/BLUEPRINT/BP_COLLECTIBLE.BP_COLLECTIBLE_C"))
  (return (or (> (Utilities|Array|Length _outactors_2) 0) (> (Utilities|Array|Length _outactors) 0))))