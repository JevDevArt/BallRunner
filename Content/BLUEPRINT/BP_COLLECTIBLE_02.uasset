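; BP_COLLECTIBLE_02 is a collectible that gets drawn into the player and disappears when something overlaps its sphere.
; The overlap plays a 2D sound and starts the Movement timeline, with no check on the overlapping actor.
; The timeline lerps location toward the player pawn, scale to zero and point light intensity to zero, each from its current value every update.
; The actor destroys itself when the timeline finishes.
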(event OnComponentBeginOverlap(Sphere)
  (params (OverlappedComponent :type Primitive%20Component%20Object%20Reference) (OtherActor :type Actor%20Object%20Reference) (OtherComp :type Primitive%20Component%20Object%20Reference) (OtherBodyIndex :type Integer) (bFromSweep :type Boolean) (SweepResult :type Hit%20Result%20Structure%20%28by%20ref%29))
  (bind _pointlight (Variables|Default|GetPointLight))
  (Audio|PlaySound2D "/Game/SOUND/Wauw.Wauw" 1.0 1.0 0.0 0 0)
  (bind (_direction _movement _scale _light_brightness) (Timeline|movement Play)
    (:Update
      (Transformation|SetActorLocation (Math|Vector|Lerp(Vector) (Transformation|GetActorLocation) (Transformation|GetActorLocation (Game|Player|GetPlayerPawn 0)) _movement) false false)
      (Transformation|SetActorScale3D (Math|Vector|Lerp(Vector) (Transformation|GetActorScale3D) "0, 0, 0" _scale))
      (Variables|Default|SetIntensity (Variables|/Script/Engine.LightComponentBase|GetIntensity _pointlight))
      (Rendering|Components|Light|SetIntensity _pointlight (Math|Float|Lerp (Variables|Default|GetIntensity) 0.0 _light_brightness)))
    (:Finished
      (Actor|DestroyActor))))

(fn ConstructionScript)