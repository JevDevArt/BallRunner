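; BP_PLATFORM is a platform that tilts about its roll axis while a BP_SPHERE overlaps its trigger.
; Trigger begin and end overlap events set and clear IsTilting after a class cast to BP_SPHERE.
; Tick uses FInterpTo to ease roll toward TiltAngle or back to level, scaled by TiltSpeed and DeltaMultiplier, holding pitch and yaw at zero.
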(event OnComponentBeginOverlap(Trigger)
  (params (OverlappedComponent :type Primitive%20Component%20Object%20Reference) (OtherActor :type Actor%20Object%20Reference) (OtherComp :type Primitive%20Component%20Object%20Reference) (OtherBodyIndex :type Integer) (bFromSweep :type Boolean) (SweepResult :type Hit%20Result%20Structure%20%28by%20ref%29))
  (bind _asbp_ball (Utilities|Casting|CastToBP_SPHEREClass (Utilities|GetClass OtherActor)))
  (Variables|Default|SetIsTilting true))

(event OnComponentEndOverlap(Trigger)
  (params (OverlappedComponent :type Primitive%20Component%20Object%20Reference) (OtherActor :type Actor%20Object%20Reference) (OtherComp :type Primitive%20Component%20Object%20Reference) (OtherBodyIndex :type Integer))
  (bind _asbp_ball (Utilities|Casting|CastToBP_SPHEREClass (Utilities|GetClass OtherActor)))
  (Variables|Default|SetIsTilting false))

(event EventTick
  (params (DeltaSeconds :type Float%20%28single-precision%29))
  (bind _deltamultiplier (Variables|Default|GetDeltaMultiplier))
  (bind _tiltspeed (Variables|Default|GetTiltSpeed))
  (bind _platform (Variables|Default|GetPlatform))
  (bind _platform_2 (Variables|Default|GetPlatform))
  (bind _returnvalue (* _deltamultiplier DeltaSeconds))
  (bind _relativerotation (Variables|/Script/Engine.SceneComponent|GetRelativeRotation _platform_2))
  (bind _roll (Math|Rotator|BreakRotator _relativerotation))
  (if (Variables|Default|GetIsTilting)
    (Transformation|SetRelativeRotation _platform (Math|Rotator|MakeRotator (Math|Interpolation|FInterpTo _roll (Variables|Default|GetTiltAngle) _returnvalue _tiltspeed) 0.0 0.0) false false)
    (else
      (Transformation|SetRelativeRotation _platform (Math|Rotator|MakeRotator (Math|Interpolation|FInterpTo _roll 0.0 _returnvalue _tiltspeed) 0.0 0.0) false false))))

(fn ConstructionScript)